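; Base interactable actor that registers itself with BP_ThirdPersonCharacter while that character stands inside its sphere trigger.
; Overlap begin and end on InteractTrigger call AddInteraction and RemoveInteraction on the character.
; The construction script configures the mesh, trigger and widget from exposed-style variables for asset, transform, radius and locations.
; ToggleUI sets prompt visibility, while Interact stores the calling character and only prints a debug string.
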(event OnComponentBeginOverlap(InteractTrigger)
  (params (OverlappedComponent :type Primitive%20Component%20Object%20Reference) (OtherActor :type Actor%20Object%20Reference) (OtherComp :type Primitive%20Component%20Object%20Reference) (OtherBodyIndex :type Integer) (bFromSweep :type Boolean) (SweepResult :type Hit%20Result%20Structure%20%28by%20ref%29))
  ;[0.15 0.15 0.15 0.5] trigger overlap
  (bind _asbp_third_person_character (Utilities|Casting|CastToBP_ThirdPersonCharacter OtherActor))
  (Default|AddInteraction _asbp_third_person_character self))

(event OnComponentEndOverlap(InteractTrigger)
  (params (OverlappedComponent :type Primitive%20Component%20Object%20Reference) (OtherActor :type Actor%20Object%20Reference) (OtherComp :type Primitive%20Component%20Object%20Reference) (OtherBodyIndex :type Integer))
  ;[0.15 0.15 0.15 0.5] trigger overlap
  (bind _asbp_third_person_character (Utilities|Casting|CastToBP_ThirdPersonCharacter OtherActor))
  (Default|RemoveInteraction _asbp_third_person_character self))

(fn ConstructionScript
  ;[0.15 0.15 0.15 0.5] Setup interactions
  (Setup|SetupMesh)
  (Setup|SetupTrigger)
  (Setup|SetupUI))

(fn SetupMesh
  ;[0.15 0.15 0.15 0.5] Setup mesh
  (Components|StaticMesh|SetStaticMesh (Variables|Default|GetInteractMesh) (Variables|Setup|GetInteractionMesh))
  (Transformation|SetRelativeTransform (Variables|Default|GetInteractMesh) (Variables|Setup|GetMeshTransform) false false))

(fn SetupTrigger
  ;[0.15 0.15 0.15 0.5] Setup trigger
  (Components|Sphere|SetSphereRadius (Variables|Default|GetInteractTrigger) (Variables|Setup|GetTriggerRadius) true)
  (Transformation|SetRelativeLocation (Variables|Default|GetInteractTrigger) (Variables|Setup|GetTriggerLocation) false false))

(fn SetupUI
  ;[0.15 0.15 0.15 0.5] Setup widget
  (Transformation|SetRelativeLocation (Variables|Default|GetInteractUI) (Variables|Setup|GetUILocation) false false))

(fn ToggleUI
  (params (Visible :type Boolean))
  ;[0.15 0.15 0.15 0.5] Set visibility
  (Rendering|SetVisibility (Variables|Default|GetInteractUI) Visible false))

(fn Interact
  (params (Character :type BP%20Third%20Person%20Character%20Object%20Reference))
  (Variables|Default|SetInteract%20character Character)
  (Development|PrintString "interact"))